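; Component that scatters pickups across its owning BP_WorldTile when play begins.
; It spawns a count of PickupClass actors derived from the tile's area times Density.
; Random indices become grid cell centers via modulo and division by tile width, with cells sized from the pickup class's default Size and offset from the tile's location.
; Spawns that would collide are skipped, so the final count can be lower.
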(event Custom|StartSpawn
  (bind _pickupclass (Variables|Default|GetPickupClass))
  (bind _size (Utilities|GetClassDefaults _pickupclass))
  (bind _returnvalue (* _size 1e+02))
  (bind _returnvalue_2 (* _returnvalue 0.5))
  (bind _asbp_world_tile (Utilities|Casting|CastToBP_WorldTile (Components|GetOwner)))
  (for _index (range 0 (- (Math|Float|Truncate (* (* (Variables|/Game/DogEatDog/LevelDesign/BP_WorldTile.BP_WorldTile_C|GetWorldSizeX _asbp_world_tile) (Variables|/Game/DogEatDog/LevelDesign/BP_WorldTile.BP_WorldTile_C|GetWorldSizeY _asbp_world_tile)) (Variables|Default|GetDensity))) 1))
    (Utilities|FlowControl|Sequence
      (:then_0
        (Game|SpawnActorfromClass (Variables|Default|GetPickupClass) (Math|Transform|MakeTransform (+ (Transformation|GetActorLocation (Components|GetOwner)) (Math|Vector|MakeVector (+ (* (Math|Integer|%(Integer) (Math|Random|RandomIntegerinRange 0 (Math|Float|Truncate (* (Variables|/Game/DogEatDog/LevelDesign/BP_WorldTile.BP_WorldTile_C|GetWorldSizeX _asbp_world_tile) (Variables|/Game/DogEatDog/LevelDesign/BP_WorldTile.BP_WorldTile_C|GetWorldSizeY _asbp_world_tile)))) (Variables|/Game/DogEatDog/LevelDesign/BP_WorldTile.BP_WorldTile_C|GetWorldSizeX _asbp_world_tile)) _returnvalue) _returnvalue_2) (+ _returnvalue_2 (* _returnvalue (/ (Math|Random|RandomIntegerinRange 0 (Math|Float|Truncate (* (Variables|/Game/DogEatDog/LevelDesign/BP_WorldTile.BP_WorldTile_C|GetWorldSizeX _asbp_world_tile) (Variables|/Game/DogEatDog/LevelDesign/BP_WorldTile.BP_WorldTile_C|GetWorldSizeY _asbp_world_tile)))) (Variables|/Game/DogEatDog/LevelDesign/BP_WorldTile.BP_WorldTile_C|GetWorldSizeX _asbp_world_tile)))) _returnvalue_2))) "DontSpawnIfColliding" "MultiplyWithRoot" (Components|GetOwner) 0)))))

(event EventBeginPlay
  (CallFunction|StartSpawn))

(event EventTick
  (params (DeltaSeconds :type Float%20%28single-precision%29)))