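; BP_WorldTile is a level-design tile that sizes its floor and moves the game camera to its center when the player enters it.
; The construction script scales the Ground mesh from WorldSizeX and WorldSizeY and fits a centered CameraTrigger box slightly inset from the tile edges.
; When BP_PLayerCharacter overlaps the trigger, it sets BP_Camera's CameraDestPosition to the tile center, keeping the camera's current height.
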(event Custom|OnComponentBeginOverlap_Event
  (params (OverlappedComponent :type Primitive%20Component%20Object%20Reference) (OtherActor :type Actor%20Object%20Reference) (OtherComp :type Primitive%20Component%20Object%20Reference) (OtherBodyIndex :type Integer) (bFromSweep :type Boolean) (SweepResult :type Hit%20Result%20Structure%20%28by%20ref%29))
  (bind _returnvalue (Transformation|GetActorLocation))
  (Utilities|Casting|CastToBP_PLayerCharacter OtherActor)
  (bind _returnvalue_2 (Actor|GetActorOfClass "/Game/DogEatDog/LevelDesign/BP_Camera.BP_Camera_C"))
  (Variables|/Game/DogEatDog/LevelDesign/BP_Camera.BP_Camera_C|SetCameraDestPosition _returnvalue_2 (Math|Vector|MakeVector (+ (.x _returnvalue) (* (/ (Variables|Default|GetWorldSizeX) 2) 1e+02)) (+ (.y _returnvalue) (* (/ (Variables|Default|GetWorldSizeY) 2) 1e+02)) (.z (Transformation|GetActorLocation _returnvalue_2)))))

(event Custom|StartCameraLogic
  (Collision|AssignOnComponentBeginOverlap (Variables|Default|GetCameraTrigger) (delegate Custom|OnComponentBeginOverlap_Event)))

(event EventBeginPlay
  (CallFunction|StartCameraLogic))

(fn ConstructionScript
  (bind _worldsizex (Variables|Default|GetWorldSizeX))
  (bind _worldsizey (Variables|Default|GetWorldSizeY))
  (bind _returnvalue (* _worldsizey 1e+02))
  (bind _returnvalue_2 (* _worldsizex 1e+02))
  (bind _returnvalue_3 (/ _returnvalue 2.0))
  (bind _returnvalue_4 (/ _returnvalue_2 2.0))
  (Transformation|SetRelativeTransform (Variables|Default|GetGround) (Math|Transform|MakeTransform (Math|Vector|MakeVector 0.0 (Math|Conversions|ToFloat(Integer) (* (Variables|Default|GetWorldSizeY) 100)) -5e+01) (Math|Rotator|MakeRotator 0.0 0.0 -9e+01) (Math|Vector|MakeVector (Math|Conversions|ToFloat(Integer) (Variables|Default|GetWorldSizeX)) (Math|Conversions|ToFloat(Integer) (Variables|Default|GetWorldSizeY)) 0.5)) false false)
  (Transformation|SetRelativeLocation (Variables|Default|GetCameraTrigger) (Math|Vector|MakeVector _returnvalue_4 _returnvalue_3 0.0) false false)
  (Components|Box|SetBoxExtent (Variables|Default|GetCameraTrigger) (Math|Vector|MakeVector (* _returnvalue_4 0.85) (* _returnvalue_3 0.85) 5e+02) true))