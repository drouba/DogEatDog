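; Pickup spawner that scatters PickupClass actors over a grid from its own location on BeginPlay, with the count set by world area times Density.
; Random cell indices, drawn from a range narrowing with each iteration, map to X/Y via a hardcoded 30-cell row, scaled by a class default.
; Colliding spawns are skipped.
; Random nodes are evaluated separately, so printed debug coordinates can differ from spawn positions.
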(event EventBeginPlay
  (bind _worldsizex (Variables|Default|GetWorldSizeX))
  (bind _worldsizey (Variables|Default|GetWorldSizeY))
  (bind _returnvalue (* _worldsizex _worldsizey))
  (for _index (range 1 (Math|Float|Truncate (* _returnvalue (Variables|Default|GetDensity))))
    (Utilities|FlowControl|Sequence
      (:then_0
        (Game|SpawnActorfromClass (Variables|Default|GetPickupClass) (Math|Transform|MakeTransform (+ (Transformation|GetActorLocation) (Math|Vector|MakeVector (- (* (* (Math|Conversions|ToFloat(Integer) (Utilities|GetClassDefaults (Variables|Default|GetPickupClass))) 1e+02) (Math|Integer|%(Integer) (Math|Random|RandomIntegerinRange _index _returnvalue) 30)) 5e+01) (- (* (/ (Math|Random|RandomIntegerinRange _index _returnvalue) 30) (* (Math|Conversions|ToFloat(Integer) (Utilities|GetClassDefaults (Variables|Default|GetPickupClass))) 1e+02)) 5e+01) 0.0))) "DontSpawnIfColliding" "MultiplyWithRoot" 0 0))
      (:then_1
        (Development|PrintString (Utilities|String|Append "X: " (Utilities|String|ToString(Float) (- (* (* (Math|Conversions|ToFloat(Integer) (Utilities|GetClassDefaults (Variables|Default|GetPickupClass))) 1e+02) (Math|Integer|%(Integer) (Math|Random|RandomIntegerinRange _index _returnvalue) 30)) 5e+01)) "Y: " (Utilities|String|ToString(Float) (- (* (/ (Math|Random|RandomIntegerinRange _index _returnvalue) 30) (* (Math|Conversions|ToFloat(Integer) (Utilities|GetClassDefaults (Variables|Default|GetPickupClass))) 1e+02)) 5e+01))))))))

(event Collision|EventActorBeginOverlap
  (params (OtherActor :type Actor%20Object%20Reference)))

(event EventTick
  (params (DeltaSeconds :type Float%20%28single-precision%29)))

(fn ConstructionScript)